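; BP_Esprit_Foule_01 is a spirit crowd Blueprint that moves its Esprits01 component when Deplacement_Esprit_Foule is triggered.
; The event stores the component's starting relative location, then plays the Up timeline, adding its track value to that location on each update.
; The Cri_Guerre_Esp_01 war cry event is empty, and a delay and a Wwise charge-cry post are left unconnected.
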(event Custom|Deplacement_Esprit_Foule
  (Utilities|FlowControl|Sequence
    (:then_0
      (Variables|Default|SetLocation_depart (Variables|/Script/Engine.SceneComponent|GetRelativeLocation (Variables|Default|Getesprits_01))))
    (:then_1
      (bind _newtrack_0 (Timeline|Up Play)
        (:Update
          (Transformation|SetRelativeLocation (Variables|Default|Getesprits_01) (+ _newtrack_0 (Variables|Default|GetLocation_depart)) false false))))))

(event Custom|Cri_Guerre_Esp_01)

(event EventBeginPlay)

(event Collision|EventActorBeginOverlap
  (params (OtherActor :type Actor%20Object%20Reference)))

(event EventTick
  (params (DeltaSeconds :type Float%20%28single-precision%29)))

(fn ConstructionScript)
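; BP_Esprit is a spirit actor that idles in place, then can cry out and flee before disappearing.
; On BeginPlay, an idle timeline offsets the Esprits01 component from its saved starting relative location.
; The flee event re-saves that location, runs movement and yaw timelines together, and destroys the actor after a short delay.
; A separate event posts the Wwise flee cry; neither event is triggered within this graph.
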(event Custom|Deplacement_Esprit_Fuite
  ;[1 1 1] Fuite de l'esprit
  (Utilities|FlowControl|Sequence
    (:then_0
      (Variables|Default|SetLocation_depart (Variables|/Script/Engine.SceneComponent|GetRelativeLocation (Variables|Default|Getesprits_01))))
    (:then_1
      (bind _newtrack_0 (Timeline|Esprit_fuite Play)
        (:Update
          (Transformation|SetRelativeLocation (Variables|Default|Getesprits_01) (+ _newtrack_0 (Variables|Default|GetLocation_depart)) false false))))
    (:then_2
      (bind _newtrack_0_2 (Timeline|Esprit_Rotation Play)
        (:Update
          (Transformation|SetRelativeRotation (Variables|Default|Getesprits_01) (Math|Rotator|MakeRotator 0.0 0.0 (.Y (Math|Vector|BreakVector _newtrack_0_2))) false false))))
    (:then_3
      (Utilities|FlowControl|Delay 5.0)
      (Actor|DestroyActor (Components|GetOwner (Variables|Default|Getesprits_01))))))

(event Custom|Cri_Fuite
  ;[1 1 1] Cri de l'esprit
  (Class|AkGameplayStatics|PostEvent "/Game/Audio/Esprit_Cri_Fuite.Esprit_Cri_Fuite" (Components|GetOwner (Variables|Default|GetEsprit_Cri_Fuite_Blueprint))))

(event EventBeginPlay
  ;[1 1 1] Esprit idle
  (Utilities|FlowControl|Sequence
    (:then_0
      (Variables|Default|SetLocation_depart (Variables|/Script/Engine.SceneComponent|GetRelativeLocation (Variables|Default|Getesprits_01))))
    (:then_1
      (bind _newtrack_0 (Timeline|Idle_Esprit Play)
        (:Update
          (Transformation|SetRelativeLocation (Variables|Default|Getesprits_01) (+ _newtrack_0 (Variables|Default|GetLocation_depart)) false false))))))

(event Collision|EventActorBeginOverlap
  (params (OtherActor :type Actor%20Object%20Reference)))

(event EventTick
  (params (DeltaSeconds :type Float%20%28single-precision%29)))

(fn ConstructionScript)
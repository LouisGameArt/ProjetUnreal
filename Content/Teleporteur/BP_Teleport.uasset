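; Teleporter platform that sends the player to the location of its TargetTp reference when the gamepad player character (BP_Player_Manette) enters its Box trigger.
; The overlap handler teleports player character 0 with zeroed rotation, then applies a half-turn local rotation.
; The construction script applies the configured material to the platform mesh.
; Variants for the first-person character and VR pawn remain in the graph but are disconnected.
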(event OnComponentBeginOverlap(Box)
  (params (OverlappedComponent :type Primitive%20Component%20Object%20Reference) (OtherActor :type Actor%20Object%20Reference) (OtherComp :type Primitive%20Component%20Object%20Reference) (OtherBodyIndex :type Integer) (bFromSweep :type Boolean) (SweepResult :type Hit%20Result%20Structure%20%28by%20ref%29))
  (bind _returnvalue (Game|GetPlayerCharacter 0))
  ;[1 1 1] TP avec BP Player Manette
  (bind _asbp_player_manette (Utilities|Casting|CastToBP_Player_Manette OtherActor))
  (if (== OtherActor (Components|GetOwner (Variables|/Script/Engine.Character|GetCapsuleComponent _asbp_player_manette)))
    (Transformation|Teleport _returnvalue (Transformation|GetActorLocation (Variables|Components|GetTarget_tp)) "0,0.000000, 0")
    (Transformation|AddActorLocalRotation _returnvalue "0,180.000000, 0" false false)))

(event EventBeginPlay)

(event Collision|EventActorBeginOverlap
  (params (OtherActor :type Actor%20Object%20Reference)))

(event EventTick
  (params (DeltaSeconds :type Float%20%28single-precision%29)))

(fn ConstructionScript
  (Rendering|Material|SetMaterial (Variables|Default|GetPlateforme) 0 (Variables|Components|GetPlateforem_Mat)))